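; Player pawn Blueprint that manages the local player's HUD: crosshair, health bar, ammo counter and wave counter.
; Tick waits until the pawn is locally controlled, then sets a one-shot flag and creates each widget on the owning player's screen.
; BeginPlay binds a death event that destroys the WidgetMarker component and removes the HUD if it was created.
; An AddHUDToPlayer helper wraps AddToPlayerScreen but is not called in this graph.
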(event Custom|OnDeathEvent_Event_0
  (Components|DestroyComponent (Variables|Default|GetWidgetMarker))
  (if (Variables|Default|GetbHasMadeUI)
    (Widget|RemovefromParent (stale EventTick _returnvalue))
    (Widget|RemovefromParent (stale EventTick _returnvalue_2))
    (Widget|RemovefromParent (stale EventTick _returnvalue_3))
    (Widget|RemovefromParent (stale EventTick _returnvalue_4))))

(event EventBeginPlay
  (EventDispatchers|AssignOnDeathEvent (delegate Custom|OnDeathEvent_Event_0)))

(event EventTick
  (params (DeltaSeconds :type Float%20%28single-precision%29))
  (if (not (Variables|Default|GetbHasMadeUI))
    (if (Pawn|IsLocallyControlled)
      (Variables|Default|SetbHasMadeUI true)
      (bind _asplayer_controller (Utilities|Casting|CastToPlayerController (Pawn|GetController)))
      (Utilities|FlowControl|Sequence
        (:then_0
          (bind _returnvalue (UserInterface|CreateWidget "/Game/UI/WBP_Crosshair.WBP_Crosshair_C" _asplayer_controller))
          (UserInterface|Viewport|AddtoPlayerScreen _returnvalue))
        (:then_1
          (bind _returnvalue_2 (UserInterface|CreateWidget "/Game/UI/WBP_HealthBar.WBP_HealthBar_C" _asplayer_controller))
          (UserInterface|Viewport|AddtoPlayerScreen _returnvalue_2))
        (:then_2
          (bind _returnvalue_3 (UserInterface|CreateWidget "/Game/UI/WBP_AmmoCounter.WBP_AmmoCounter_C" _asplayer_controller))
          (UserInterface|Viewport|AddtoPlayerScreen _returnvalue_3))
        (:then_3
          (bind _returnvalue_4 (UserInterface|CreateWidget "/Game/UI/WBP_WaveCounter.WBP_WaveCounter_C" _asplayer_controller))
          (UserInterface|Viewport|AddtoPlayerScreen _returnvalue_4))))))

(fn ConstructionScript)

(fn AddHUDtoPlayer
  (params (HUDElement :type User%20Widget%20Object%20Reference))
  (UserInterface|Viewport|AddtoPlayerScreen HUDElement))