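; BP_RollerBot is an AI bot that moves erratically as a physics-driven rolling mesh.
; Each tick, it applies a random-direction acceleration with a slight upward bias to its mesh, ignoring mass, until its Exploded flag is set.
; Rolling audio volume scales with current speed every tick, even after exploding.
; The graph contains no targeting or explosion logic, and the construction script is empty.
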(event EventTick
  (params (DeltaSeconds :type Float%20%28single-precision%29))
  (Audio|Components|Audio|SetVolumeMultiplier (Variables|Default|GetRollingAudio) (Math|Float|MapRangeClamped (Math|Vector|VectorLength (Transformation|GetVelocity)) 1e+01 1e+03 0.0 2.0) :!class /Script/Engine.AudioComponent)
  (if (not (Variables|Default|GetbExploded))
    (Physics|AddForce (Variables|Default|GetMeshComponent) (+ (* (Math|Random|RandomUnitVector) (Math|Random|RandomFloatinRange 1e+03 5e+03)) "0, 0,100.000000") "None" true)))

(fn ConstructionScript)