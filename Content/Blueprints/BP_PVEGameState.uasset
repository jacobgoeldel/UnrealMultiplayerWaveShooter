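; PVE game state that reacts to wave state changes in a wave-based match.
; WaveStateChanged shows a WBP_PopupMessage on each player controller's screen for preparing, wave number and game over, while a win only prints a debug string.
; The preparing phase also respawns all spectators, in a loop nested inside the per-controller loop.
; AddHUDToEachPlayer passes a HUD element to every BP_Player.
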(event EventWaveStateChanged
  (params (newState :type EWaveState%20Enum :default "Preparing") (oldState :type EWaveState%20Enum :default "Preparing"))
  (switch Utilities|FlowControl|Switch|SwitchonEWaveState newState
    (:Preparing
      (bind _outactors (Actor|GetAllActorsOfClass "/Game/Blueprints/BP_PlayerController.BP_PlayerController_C"))
      (for _array_element _outactors
        (bind _returnvalue (UserInterface|CreateWidget "/Game/UI/WBP_PopupMessage.WBP_PopupMessage_C" _array_element))
        (Rendering|Components|TextRender|SetText (Variables|/Game/UI/WBP_PopupMessage.WBP_PopupMessage_C|GetTextBlock_0 _returnvalue) "Prepare For Next Wave")
        (UserInterface|Viewport|AddtoPlayerScreen _returnvalue)
        (bind _outactors_2 (Actor|GetAllActorsOfClass "/Game/Blueprints/BP_Spectator.BP_Spectator_C"))
        (for _array_element_2 _outactors_2
          (bind _asbp_spectator (Utilities|Casting|CastToBP_Spectator _array_element_2))
          (Default|Respawn _asbp_spectator))))
    (:WaveInProgress
      (bind _outactors_3 (Actor|GetAllActorsOfClass "/Game/Blueprints/BP_PlayerController.BP_PlayerController_C"))
      (for _array_element_3 _outactors_3
        (bind _returnvalue_2 (UserInterface|CreateWidget "/Game/UI/WBP_PopupMessage.WBP_PopupMessage_C" _array_element_3))
        (Rendering|Components|TextRender|SetText (Variables|/Game/UI/WBP_PopupMessage.WBP_PopupMessage_C|GetTextBlock_0 _returnvalue_2) (Utilities|Text|ToText(String) (Utilities|String|Append "Wave " (Utilities|String|ToString(Integer) (Variables|Default|GetWave)))))
        (UserInterface|Viewport|AddtoPlayerScreen _returnvalue_2)))
    (:Gameover
      (bind _outactors_4 (Actor|GetAllActorsOfClass "/Game/Blueprints/BP_PlayerController.BP_PlayerController_C"))
      (for _array_element_4 _outactors_4
        (bind _returnvalue_3 (UserInterface|CreateWidget "/Game/UI/WBP_PopupMessage.WBP_PopupMessage_C" _array_element_4))
        (Rendering|Components|TextRender|SetText (Variables|/Game/UI/WBP_PopupMessage.WBP_PopupMessage_C|GetTextBlock_0 _returnvalue_3) "Game Over")
        (UserInterface|Viewport|AddtoPlayerScreen _returnvalue_3)))
    (:GameWon
      (Development|PrintString "Won the match!" true true "(R=0.000000,G=0.660000,B=1.000000,A=1.000000)" 1e+01))))

(fn ConstructionScript)

(fn AddHUDtoEachPlayer
  (params (HUDElement :type User%20Widget%20Object%20Reference))
  (bind _outactors (Actor|GetAllActorsOfClass "/Game/Blueprints/BP_Player.BP_Player_C"))
  (for _array_element _outactors
    (Default|AddHUDtoPlayer _array_element HUDElement)))