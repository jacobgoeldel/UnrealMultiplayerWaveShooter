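; BP_Spectator is a spectator that respawns its controller as a new player character.
; Respawn runs the EQS_FindPlayerSpawn environment query from itself, picking randomly among the best 25% of results, and binds a callback for completion.
; On query success, RespawnPointFoundEvent spawns BP_Player at the found location, has the spectator's controller possess it, then destroys the spectator.
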(event Custom|RespawnPointFoundEvent
  (params (QueryInstance :type Env%20Query%20Instance%20Blueprint%20Wrapper%20Object%20Reference) (QueryStatus :type EEnvQueryStatus%20Enum :default "Processing"))
  (switch Utilities|FlowControl|Switch|SwitchonEEnvQueryStatus QueryStatus
    (:Success
      (bind _resultlocations (AI|EQS|GetQueryResultsasLocations QueryInstance))
      (bind _returnvalue (Game|SpawnActorfromClass "/Game/Blueprints/BP_Player.BP_Player_C" (Math|Transform|MakeTransform (Utilities|Array|Get(acopy) _resultlocations)) "AdjustIfPossibleButAlwaysSpawn" 0 0))
      (Pawn|Possess (Pawn|GetController) _returnvalue)
      (Actor|DestroyActor))))

(fn ConstructionScript)

(fn Respawn
  (bind _returnvalue (AI|EQS|RunEQSQuery "/Game/Blueprints/EQS_FindPlayerSpawn.EQS_FindPlayerSpawn" self "RandomBest25Pct"))
  (EventDispatchers|BindEventtoOnQueryFinishedEvent _returnvalue (EventDispatchers|CreateEvent :!event Custom|RespawnPointFoundEvent)))